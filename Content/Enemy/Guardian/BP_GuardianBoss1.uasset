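; Guardian boss enemy that roams random nearby points, chases the player on sight and deals melee damage on reaching them, with a cooldown.
; Pawn sensing starts the chase and its music; a retriggerable delay returns it to roaming and fades the music once sight is lost.
; It binds to state changes on its crystals and, when the check finds them all on, plays a death sound and destroys itself.
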(event OnSeePawn(PawnSensing)
  (params (Pawn :type Pawn%20Object%20Reference))
  (Utilities|FlowControl|Sequence
    (:then_0
      (CallFunction|FollowPlayer)
      (Utilities|FlowControl|DoOnce false :!label _label
        (:Completed
          (bind _returnvalue (Audio|SpawnSound2D "/Game/Sounds/ChaseThemeWIP.ChaseThemeWIP" 1.0 1.0 0.0 0))
          (Variables|Default|SetChaseSong _returnvalue)
          (goto _label_2 Reset))))
    (:then_1
      (Utilities|FlowControl|RetriggerableDelay 1.0)
      (CallFunction|Roam)
      (Utilities|FlowControl|DoOnce false :!label _label_2
        (:Completed
          (Audio|Components|Audio|FadeOut (Variables|Default|GetChaseSong) 0.5 0.0 "Linear" :!class /Script/Engine.AudioComponent)
          (goto _label Reset))))))

(event Custom|OnCrystalStateChanged_Event
  (CallFunction|CustomEventBoss)
  (Development|PrintString "Guardian's Deactivation Switch!"))

(event Custom|Roam
  (Variables|/Script/Engine.CharacterMovementComponent|SetMaxWalkSpeed (Variables|Character|GetCharacterMovement) 4e+02)
  (AI|AIMoveTo self (.RandomLocation (AI|Navigation|GetRandomReachablePointinRadius (Transformation|GetActorLocation) 1.5e+03 0 0)) 0 5.0 false
    (:OnSuccess
      (Utilities|FlowControl|Delay 2.0)
      (CallFunction|Roam))))

(event Custom|followPlayer
  (Variables|Default|SetcanAttack? true)
  (Variables|/Script/Engine.CharacterMovementComponent|SetMaxWalkSpeed (Variables|Character|GetCharacterMovement) 5e+02)
  (AI|AIMoveTo self "0, 0, 0" (Game|GetPlayerCharacter 0) 7e+01 false
    (:OnSuccess
      (if (Variables|Default|GetcanAttack?)
        (Variables|Default|SetcanAttack? false)
        (Utilities|FlowControl|DoOnce false :!label _label
          (:Completed
            (CallFunction|AttackPlayer)
            (Development|PrintString "Attacked Player")
            (Utilities|FlowControl|Delay 2.0)
            (Variables|Default|SetcanAttack? true)
            (Variables|/Script/Engine.CharacterMovementComponent|SetMaxWalkSpeed (Variables|Character|GetCharacterMovement) 4e+02)
            (goto _label Reset)))))))

(event Custom|AttackPlayer
  (bind _asbp_player_char (Utilities|Casting|CastToBP_PlayerChar (Game|GetPlayerCharacter 0)))
  (Game|Damage|ApplyDamage _asbp_player_char 2e+01 0 self)
  (Variables|Default|SetcanAttack? false))

(event Custom|CustomEventBoss
  (bind _chasesong (Variables|Default|GetChaseSong))
  (Development|PrintString "Checking")
  (if (Variables|Default|GetisCrystals)
    (Variables|Default|SetAllOn true)
    (bind _array_element (Utilities|Array|ForEachLoopwithBreak (Variables|Default|GetCystals) :!label _label)
      (:LoopBody
        (if (not (Variables|/Game/Interactables/BP_Crystal.BP_Crystal_C|GetIsON _array_element))
          (Variables|Default|SetAllOn false)
          (goto _label Break)))
      (:Completed
        (if (Variables|/Game/Interactables/BP_Crystal.BP_Crystal_C|GetIsON _array_element)
          (Variables|Default|SetisCompleted true)
          (Development|PrintString "OH NO IM DEAD")
          (if (Utilities|IsValid _chasesong)
            (Audio|Components|Audio|FadeOut _chasesong 0.5 0.0 "Linear" :!class /Script/Engine.AudioComponent))
          (Audio|PlaySound2D "/Game/Sounds/Death.Death" 1.0 1.0 0.0 0 0)
          (Actor|DestroyActor)
          (else
            (Variables|Default|SetisCompleted false)))))))

(event EventBeginPlay
  (Utilities|FlowControl|Sequence
    (:then_0
      (for _array_element (Variables|Default|GetCystals)
        (EventDispatchers|BindEventtoOnCrystalStateChanged _array_element (delegate Custom|OnCrystalStateChanged_Event))))
    (:then_1
      (CallFunction|Roam)
      (Development|PrintString "Roaming"))))

(event EventTick
  (params (DeltaSeconds :type Float%20%28single-precision%29)))

(fn ConstructionScript)

(fn CrystalCheck)