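; BP_Crystal is an interactable crystal that toggles between on and off states through the INTInteract interaction event.
; Each toggle flips IsON, swaps the Cone mesh material, prints a debug message and calls OnCrystalStateChanged to broadcast the change.
; Turning it on also plays a 2D sound.
; The construction script applies the on material when IsON is preset, so the starting state shows in the editor.
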(event EventBeginPlay)

(event Collision|EventActorBeginOverlap
  (params (OtherActor :type Actor%20Object%20Reference)))

(event EventTick
  (params (DeltaSeconds :type Float%20%28single-precision%29)))

(event EventINTInteract
  (params (PlayerRef :type BP%20Player%20Char%20Object%20Reference))
  (if (Variables|Default|GetIsON)
    (Rendering|Material|SetMaterial (Variables|Default|GetCone) 0 "/Game/Materials/MAT_CrystalOff.MAT_CrystalOff")
    (Variables|Default|SetIsON false)
    (Development|PrintString "Crystal Off!")
    (Default|CallOnCrystalStateChanged)
    (else
      (Rendering|Material|SetMaterial (Variables|Default|GetCone) 0 "/Game/Materials/MAT_CrystalOn.MAT_CrystalOn")
      (Variables|Default|SetIsON true)
      (Audio|PlaySound2D "/Game/Sounds/isolated_menu_sounds_2-hovers_and_selects.isolated_menu_sounds_2-hovers_and_selects" 1.0 1.0 0.0 0 0)
      (Development|PrintString "Crystal On!")
      (Default|CallOnCrystalStateChanged))))

(fn ConstructionScript
  (if (Variables|Default|GetIsON)
    (Rendering|Material|SetMaterial (Variables|Default|GetCone) 0 "/Game/Materials/MAT_CrystalOn.MAT_CrystalOn")))