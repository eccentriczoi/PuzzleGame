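; BP_AnnounceWin is a trigger volume that announces the player's victory and ends the boss encounter.
; The first overlap by BP_PlayerChar plays a win sound, sets IsWin, calls MainMenuKey on the player and prints a congratulations message offering a return to the main menu.
; It then tells BossRoom to swap to its end music and, after a short delay, teleports the player to the world origin, described as the sandbox.
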(event OnComponentBeginOverlap(Box)
  (params (OverlappedComponent :type Primitive%20Component%20Object%20Reference) (OtherActor :type Actor%20Object%20Reference) (OtherComp :type Primitive%20Component%20Object%20Reference) (OtherBodyIndex :type Integer) (bFromSweep :type Boolean) (SweepResult :type Hit%20Result%20Structure%20%28by%20ref%29))
  (bind _asbp_player_char (Utilities|Casting|CastToBP_PlayerChar OtherActor))
  (if true
    (Utilities|FlowControl|DoOnce false
      (:Completed
        (Audio|PlaySound2D "/Game/Sounds/WinPuzzle.WinPuzzle" 1.0 1.0 0.0 0 0)
        (Variables|Default|SetisWin? true)
        (bind _asbp_player_char_2 (Utilities|Casting|CastToBP_PlayerChar _asbp_player_char))
        (Default|MainMenuKey _asbp_player_char_2)
        (Development|PrintString "Congrats You Won!  
You will be teleporting to sandbox! 
Press ENTER to go back to Main Menu")
        (Default|SwapMusicEnd (Variables|Default|GetBossRoom))
        (Utilities|FlowControl|Delay 4.0)
        (Transformation|SetActorLocation OtherActor "0, 0, 0" false false)))))

(event EventBeginPlay)

(event EventTick
  (params (DeltaSeconds :type Float%20%28single-precision%29)))

(fn ConstructionScript)