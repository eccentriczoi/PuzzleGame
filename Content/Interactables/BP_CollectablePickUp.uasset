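; BP_CollectablePickUp is an interactable pickup that bobs in place and grants score and health to the player.
; BeginPlay loops the cube's vertical bob by chaining two timelines, one forward and one reversed.
; INTInteract adds a point, casts to BP_PlayerChar and plays a sound.
; Only when healing stays within maximum health does it raise health, update the health bar and destroy itself, so otherwise it remains collectable.
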(event EventBeginPlay
  (bind _float (Timeline|FloatAnim Play)
    (:Update
      (Transformation|SetRelativeLocation (Variables|Default|GetCube) (Math|Vector|MakeVector 0.0 0.0 (.z _float)) false false))
    (:Finished
      (bind _float_2 (Timeline|Timeline ReverseFromEnd)
        (:Update
          (Transformation|SetRelativeLocation (Variables|Default|GetCube) (Math|Vector|MakeVector 0.0 0.0 (.z _float_2)) false false))
        (:Finished
          (Timeline|FloatAnim PlayFromStart))))))

(event Collision|EventActorBeginOverlap
  (params (OtherActor :type Actor%20Object%20Reference)))

(event EventTick
  (params (DeltaSeconds :type Float%20%28single-precision%29)))

(event EventINTInteract
  (params (PlayerRef :type BP%20Player%20Char%20Object%20Reference))
  (Default|AddScore PlayerRef 1)
  (bind _asbp_player_char (Utilities|Casting|CastToBP_PlayerChar PlayerRef))
  (Audio|PlaySound2D "/Game/Sounds/SelectSFX.SelectSFX" 1.0 1.0 0.0 0 0)
  (if (<= (+ (Variables|/Game/Player/BP_PlayerChar.BP_PlayerChar_C|GetHealth PlayerRef) 1e+01) 1e+02)
    (bind _output_get (Variables|/Game/Player/BP_PlayerChar.BP_PlayerChar_C|SetHealth _asbp_player_char (+ (Variables|/Game/Player/BP_PlayerChar.BP_PlayerChar_C|GetHealth PlayerRef) 1e+01)))
    (Default|UpdateHealthBar (Variables|/Game/Player/BP_PlayerChar.BP_PlayerChar_C|GetHealthBarRefernce PlayerRef) _output_get)
    (Actor|DestroyActor)))

(fn ConstructionScript)